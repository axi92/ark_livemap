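; Location flag structure that shows a toggleable range mesh and limits how many flags a tribe can build.
; On BeginPlay it polls the HTTP location singleton every second until its INI is loaded, then caches the range scale.
; Placement checks count same-team, non-preview flags against the limit, with debug prints.
; Tribe members and admins get a show/hide menu entry, and the OnRep handler scales and hides the mesh.
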(event `self.ReceiveBeginPlay`
  (`parent.ReceiveBeginPlay`)
  (bind _returnvalue (`GameplayStatics.GetActorOfClass` null "/ark_livemap/Singleton_HTTPLocation_Actor.Singleton_HTTPLocation_Actor_C" :!label _label))
  (`/Engine/EditorBlueprintResources/StandardMacros.IsValid` _returnvalue
    (:`Is Valid`
      (if (`/ark_livemap/Singleton_HTTPLocation_Actor.bIniLoaded` _returnvalue)
        (set `self.FlagRangeMeshScaleLocal` (`/ark_livemap/Singleton_HTTPLocation_Actor.FlagRangeMeshScale` _returnvalue) true)
        (else
          (`KismetSystemLibrary.Delay` null 1.0 :!label _label_2)
          (goto _label))))
    (:`Is Not Valid`
      (goto _label_2))))

(fn `BPGetMultiUseEntries`
  (params (ForPC :type "PlayerController Object Reference") (MultiUseEntries :type "Array of MultiUseEntry Structure (by ref)"))
  (returns (ReturnValue :type "Array of MultiUseEntry Structure"))
  (locals (MultiUseBuffer_1 :type "Array of MultiUseEntry Structure"))
  (bind _flagrangemeshscalelocal (`self.FlagRangeMeshScaleLocal`))
  (bind _multiusebuffer_1 (`local.MultiUseBuffer_1`))
  (bind _asshooter_player_controller (cast `ShooterPlayerController` ForPC))
  (bind _returnvalue (`self.AllowStructureAccess` _asshooter_player_controller)) ; If player is in tribe
  (if (or _returnvalue (`PrimalPlayerController.bIsAdmin` _asshooter_player_controller))
    (set `local.MultiUseBuffer_1` MultiUseEntries)
    (`KismetArrayLibrary.Array_Add` _multiusebuffer_1 (make `MultiUseEntry` null (`KismetMathLibrary.SelectString` (`KismetStringLibrary.BuildString_Double` "Show range" " " _flagrangemeshscalelocal) (`KismetStringLibrary.BuildString_Double` "Hide range" " " _flagrangemeshscalelocal) (`self.IsRangeIndicatorHidden`)) (`self.MultiUseIndex_ToggleRangeIndicator`)))
    (return _multiusebuffer_1)))

(fn `BPIsAllowedToBuild`
  (params (OutPlacementData :type "PlacementData Structure (by ref)") (CurrentAllowedReason :type Integer))
  (returns (ReturnValue :type Integer))
  (locals (StructureCount :type Integer))
  (bind _structurecount (`local.StructureCount`))
  (bind _targetingteam (`Actor.TargetingTeam`))
  (bind _returnvalue (`KismetMathLibrary.Conv_BoolToInt` (not (> _structurecount 1))))
  (`KismetSystemLibrary.PrintString` null "tribe placing:")
  (`KismetSystemLibrary.PrintString` null (`KismetStringLibrary.Conv_IntToString` _targetingteam))
  (`KismetSystemLibrary.PrintString` null "current allowed reason")
  (`KismetSystemLibrary.PrintString` null (`KismetStringLibrary.Conv_IntToString` CurrentAllowedReason))
  (bind _asactor (castclass `Actor` (`GameplayStatics.GetObjectClass` self))
    (:`then`
      (bind _outactors (`GameplayStatics.GetAllActorsOfClass` null _asactor))
      (for _array_element _outactors
        (bind _asprimal_structure (cast `PrimalStructure` _array_element))
        (`KismetSystemLibrary.PrintString` null "isPreview:")
        (bind _bispreviewstructure (`PrimalStructure.bIsPreviewStructure` _asprimal_structure))
        (`KismetSystemLibrary.PrintString` null (`KismetStringLibrary.Conv_BoolToString` _bispreviewstructure))
        (`KismetSystemLibrary.PrintString` null "team:")
        (bind _targetingteam_2 (`Actor.TargetingTeam` _asprimal_structure))
        (`KismetSystemLibrary.PrintString` null (`KismetStringLibrary.Conv_IntToString` _targetingteam_2))
        (if _bispreviewstructure
          _
          (elif (== _targetingteam _targetingteam_2)
            (set `local.StructureCount` (+ (`local.StructureCount`) 1)))))
      (`KismetSystemLibrary.PrintString` null "structure count:")
      (`KismetSystemLibrary.PrintString` null (`KismetStringLibrary.Conv_IntToString` _structurecount))
      (`KismetSystemLibrary.PrintString` null "return value")
      (`KismetSystemLibrary.PrintString` null (`KismetStringLibrary.Conv_IntToString` _returnvalue))
      (return _returnvalue) ; allowed = 1
    )
    (:`CastFailed`
      (`KismetSystemLibrary.PrintString` null "Cast failed BPIsAllowedToBuildEx on LocationFlag_BP"))))

(fn `BPTryMultiUse`
  (params (ForPC :type "PlayerController Object Reference") (UseIndex :type Integer))
  (returns (ReturnValue :type Boolean))
  (`|ExecutionSequence`
    (:`then_0`
      (switch `int` UseIndex ; Range
        (:`17844`
          (set `self.IsRangeIndicatorHidden` (not (`self.IsRangeIndicatorHidden`)) true))))
    (:`then_1`
      (return false))))

(fn `OnRep_IsRangeIndicatorHidden`
  (bind _returnvalue (`KismetSystemLibrary.MakeLiteralDouble` (`self.FlagRangeMeshScaleLocal`)))
  (`/Engine/EditorBlueprintResources/StandardMacros.Can Execute Cosmetic Events`
    (:`True`
      (`SceneComponent.SetRelativeScale3D` (`self.FlagRangeMesh`) (`KismetMathLibrary.MakeVector` _returnvalue _returnvalue _returnvalue))
      (`SceneComponent.SetHiddenInGame` (`self.FlagRangeMesh`) (`self.IsRangeIndicatorHidden`) false true))))

(fn `UserConstructionScript`)