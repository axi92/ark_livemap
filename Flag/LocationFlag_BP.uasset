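; LocationFlag_BP is a placeable flag structure, apparently for ARK, that limits how many flags each tribe can build.
; Its build check scans actors of its class, counts non-preview ones on the same team, and disallows placement when the count exceeds one, with debug prints throughout.
; A multi-use entry for toggling survivor position is stubbed: its label always reads "Hide" and its handler only fetches player data, returning false.
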(fn ConstructionScript)

(fn BPIsAllowedtoBuild
  (params (OutPlacementData :type Placement%20Data%20Structure%20%28by%20ref%29) (CurrentAllowedReason :type Integer))
  (bind _self self)
  (bind _targetingteam (Variables|/Script/Engine.Actor|GetTargetingTeam _self))
  (Development|PrintString "tribe placing:")
  (Development|PrintString (Utilities|String|ToString(Integer) _targetingteam))
  (Development|PrintString "current allowed reason")
  (Development|PrintString (Utilities|String|ToString(Integer) CurrentAllowedReason))
  (bind _asactor (Utilities|Casting|CastToActorClass (Utilities|GetClass self))
    (:then
      (bind _outactors (Actor|GetAllActorsOfClass _asactor))
      (for _array_element _outactors
        (bind _asprimalstructure (Utilities|Casting|CastToPrimalStructure _array_element))
        (Development|PrintString "isPreview:")
        (Development|PrintString (Utilities|String|ToString(Boolean) (Variables|/Script/ShooterGame.PrimalStructure|GetbIsPreviewStructure _asprimalstructure)))
        (Development|PrintString "team:")
        (Development|PrintString (Utilities|String|ToString(Integer) (Variables|/Script/Engine.Actor|GetTargetingTeam _asprimalstructure)))
        (if (not (Variables|/Script/ShooterGame.PrimalStructure|GetbIsPreviewStructure _asprimalstructure))
          (if (== _targetingteam (Variables|/Script/Engine.Actor|GetTargetingTeam _asprimalstructure))
            (LocalVariables|SetStructureCount (+ (LocalVariables|GetStructureCount) 1)))))
      (Development|PrintString "structure count:")
      (Development|PrintString (Utilities|String|ToString(Integer) (LocalVariables|GetStructureCount)))
      (Development|PrintString "return value")
      (Development|PrintString (Utilities|String|ToString(Integer) (Math|Conversions|ToInteger(Boolean) (not (> (LocalVariables|GetStructureCount) 1)))))
      (return (Math|Conversions|ToInteger(Boolean) (not (> (LocalVariables|GetStructureCount) 1)))))
    (:CastFailed
      (Development|PrintString "Cast failed BPIsAllowedToBuildEx on LocationFlag_BP"))))

(fn BPGetMultiUseEntries
  (params (ForPC :type Player%20Controller%20Object%20Reference) (MultiUseEntries :type Array%20of%20Multi%20Use%20Entry%20Structures))
  (LocalVariables|SetMultiUseBuffer_1 MultiUseEntries)
  (Utilities|Array|Add (LocalVariables|GetMultiUseBuffer_1) (Utilities|Struct|MakeMultiUseEntry 0 (Utilities|String|SelectString "Hide survivor position" "Show survivor position" true) (Variables|Default|GetMultiUseIndex_ToggleSurvivorPos)))
  (return (LocalVariables|GetMultiUseBuffer_1)))

(fn BPTryMultiUse
  (params (ForPC :type Player%20Controller%20Object%20Reference) (UseIndex :type Integer))
  (if true
    (bind _returnvalue (Class|ShooterCharacter|GetPlayerData (Class|VictoryCore|GetShooterCharacterfromController ForPC)))
    (Class|PrimalPlayerData|GetUniqueIdString _returnvalue)
    (return false)))